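; AC_Raycast is a component that casts a line trace from the player camera along its view direction.
; Every tick it traces on the Visibility channel from the first player's camera manager location out to TraceRange.
; The trace draws timed debug lines, and its hit result is not used.
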(event EventTick
  (params (DeltaSeconds :type Float%20%28single-precision%29))
  (bind _returnvalue (Game|GetPlayerCameraManager 0))
  (bind _output_get (Variables|Default|SetEndLocation (+ (Transformation|GetWorldLocation (Variables|/Script/Engine.Actor|GetRootComponent _returnvalue)) (* (Transformation|GetActorForwardVector _returnvalue) (Variables|Default|GetTraceRange)))))
  (bind _output_get_2 (Variables|Default|SetStartLocation (Transformation|GetActorLocation _returnvalue)))
  (Collision|LineTraceByChannel _output_get_2 _output_get "TraceTypeQuery1" false 0 "ForDuration"))